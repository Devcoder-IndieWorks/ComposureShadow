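; Composure CG capture element that builds a foreground render list relative to a mask actor.
; It overrides the target actor list, keeping only the parent's actors whose origins are no farther from the target camera than the mask actor, using squared distances.
; Without a valid mask actor or camera, the override skips this filtering entirely.
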(fn ConstructionScript
  (|CallParentFunction))

(fn ConstructTargetActorsList
  (Utilities|IsValid (Variables|Composure|MaskCapture|GetMaskActor)
    (:Is%20Valid
      (bind _output_get (LocalVariables|SetTargetCamera (Class|CompositingElement|FindTargetCamera)))
      (Utilities|IsValid _output_get
        (:Is%20Valid
          (Utilities|FlowControl|Sequence
            (:then_0
              (LocalVariables|SetDistanceToMaskActor (Class|KismetMathLibrary|VectorDistanceSquared (Transformation|GetActorLocation (LocalVariables|GetTargetCamera)) (Transformation|GetActorLocation (Variables|Composure|MaskCapture|GetMaskActor)))))
            (:then_1
              (bind (_bisempty _targetedactors) (|CallParentFunction))
              (if (not _bisempty)
                (for _array_element _targetedactors
                  (bind _output_get_2 (LocalVariables|SetDistanceToActor (Class|KismetMathLibrary|VectorDistanceSquared (Transformation|GetActorLocation (LocalVariables|GetTargetCamera)) (Transformation|GetActorLocation _array_element))))
                  (if (<= _output_get_2 (LocalVariables|GetDistanceToMaskActor))
                    (Utilities|Array|Add (LocalVariables|GetActorList) _array_element)))))
            (:then_2
              (return false (LocalVariables|GetActorList) "NewEnumerator0"))))))))